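; BP_Enemy_Light is an enemy that displays its health and armour and can drop loot when it dies.
; On BeginPlay it rolls a random armour value and passes it to its BP_Enemy_Widget.
; Tick refreshes the health and armour text renders and polls for zero health.
; On death it usually spawns a BP_LootDrop above itself with a base loot multiplier, then destroys itself.
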(event `self.ReceiveBeginPlay`
  (bind _output_get (set `self.Armour` (`KismetMathLibrary.RandomIntegerInRange` 0 50)))
  (bind _asbp_enemy_widget (cast `/Game/Blueprints/BP_Enemy_Widget` (`WidgetComponent.GetUserWidgetObject` (`self.UI`))))
  (`/Game/Blueprints/BP_Enemy_Widget.Enemy_Armour` _asbp_enemy_widget _output_get))

(event `self.ReceiveTick`
  (params (DeltaSeconds :type "Float (single-precision)"))
  (bind (_returnvalue_location _returnvalue_rotation _returnvalue_scale) (`KismetMathLibrary.BreakTransform` (`self.GetTransform`)))
  (`TextRenderComponent.K2_SetText` (`self.Health_Render`) (`KismetTextLibrary.Conv_DoubleToText` (`self.Health`) "HalfToEven"))
  (`TextRenderComponent.K2_SetText` (`self.Armour_Render`) (`KismetTextLibrary.Conv_IntToText` (`self.Armour`)))
  (if (<= (`self.Health`) 0.0)
    (if (`KismetMathLibrary.RandomBoolWithWeight` 0.8)
      (bind _returnvalue (`|SpawnActorFromClass` "/Game/Blueprints/BP_LootDrop.BP_LootDrop_C" (`KismetMathLibrary.MakeTransform` (+ _returnvalue_location (0.0 0.0 500.0)) _returnvalue_rotation _returnvalue_scale) "Undefined" "OverrideRootScale" null null))
      (set `/Game/Blueprints/BP_LootDrop.Loot_Multiplier` 1.0 _returnvalue))
    (`self.K2_DestroyActor`)))

(fn `UserConstructionScript`)