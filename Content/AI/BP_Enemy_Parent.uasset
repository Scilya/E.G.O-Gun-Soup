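; Base enemy Blueprint that detects the player, fires projectiles and can drop loot on death.
; Pawn sensing stores the player reference, and Agro fires projectiles using delay and damage from the child-actor weapon.
; Non-lethal hits record a damage source, cleared on arrival, while death notifies the HUD with the Boss flag.
; Construction initializes health and armour, and Tick turns the health widget toward the screen-center camera point.
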(event `self.ReceiveBeginPlay`
  (bind _asbp_enemy_widget (cast `/Game/Blueprints/BP_Enemy_Widget` (`WidgetComponent.GetUserWidgetObject` (`self.Health_Display`))))
  (`/Game/Blueprints/BP_Enemy_Widget.Enemy_Armour` _asbp_enemy_widget (`self.Armour`))
  (bind _asweapon_generation_test (cast `/Game/Actors/WeaponGenerationTest` (`ChildActorComponent.ChildActor` (`self.Weapon`))))
  (set `self.Weapon_Ref` _asweapon_generation_test)
  (add `PawnSensingComponent.OnSeePawn` (`self.PawnSensing`) (delegate `OnPawnSeen`)))

(event `OnDamage`
  (params (DirectionOfDamage :type "Vector Structure"))
  (if (<= (`self.Health`) 0.0)
    (`self.OnDestroy` null)
    (else
      (set `self.Damage_Source` DirectionOfDamage))))

(event `OnPawnSeen`
  (params (Pawn :type "Pawn Object Reference"))
  (bind _asbp_player (cast `/Game/Blueprints/BP_Player` Pawn)
    (:`then`
      (set `self.Player_Seen?` true)
      (set `self.Player_Ref` _asbp_player))
    (:`CastFailed`
      (set `self.Player_Seen?` false))))

(event `Agro`
  (params (`Player Ref` :type "Actor Object Reference"))
  (bind _gun_point (`self.Gun_Point`))
  (`KismetSystemLibrary.Delay` (/ 2.0 (`/Game/Actors/WeaponGenerationTest.Fire_Rate` (`self.Weapon_Ref`))))
  (`SceneComponent.K2_SetWorldRotation` _gun_point (`KismetMathLibrary.FindLookAtRotation` (`SceneComponent.K2_GetComponentLocation` _gun_point) (+ (`self.K2_GetActorLocation` `Player Ref`) (0.0 0.0 400.0))) false false)
  (bind _returnvalue (`|SpawnActorFromClass` "/Game/AI/BP_EnemyProjectile.BP_EnemyProjectile_C" (`SceneComponent.K2_GetComponentToWorld` _gun_point) "Undefined" "OverrideRootScale" null null))
  (`/Engine/EditorBlueprintResources/StandardMacros.IsValid` _returnvalue
    (:`Is Valid`
      (set `/Game/AI/BP_EnemyProjectile.Damage` (`/Game/Actors/WeaponGenerationTest.Damage` (`self.Weapon_Ref`)) _returnvalue))))

(event `OnDestroy`
  (params (DestroyedActor :type "Actor Object Reference"))
  (bind (_returnvalue_location _returnvalue_rotation _returnvalue_scale) (`KismetMathLibrary.BreakTransform` (`self.GetTransform`)))
  (if (`KismetMathLibrary.RandomBoolWithWeight` (`self.Drop_Weight`))
    (bind _returnvalue (`|SpawnActorFromClass` "/Game/Blueprints/BP_Interactable_Loot.BP_Interactable_Loot_C" (`KismetMathLibrary.MakeTransform` (+ _returnvalue_location (0.0 0.0 500.0)) _returnvalue_rotation _returnvalue_scale) "Undefined" "OverrideRootScale" null null))
    (set `/Game/Blueprints/BP_Interactable_Loot.Loot_Multiplier` (`self.Loot_Multiplier`) _returnvalue))
  (bind _foundwidgets (`WidgetBlueprintLibrary.GetAllWidgetsOfClass` "/Game/Blueprints/BP_Widget.BP_Widget_C"))
  (for _array_element _foundwidgets
    (`/Game/Blueprints/BP_Widget.Enemy_Killed` _array_element (`self.Boss?`))
    (`self.K2_DestroyActor`)))

(event `self.ReceiveTick`
  (params (DeltaSeconds :type "Float (single-precision)"))
  (bind _returnvalue (`GameplayStatics.GetPlayerController` 0))
  (bind _health_display (`self.Health_Display`))
  (bind (_sizex _sizey) (`PlayerController.GetViewportSize` _returnvalue))
  (`SceneComponent.K2_SetWorldRotation` _health_display (`KismetMathLibrary.FindLookAtRotation` (`SceneComponent.K2_GetComponentLocation` _health_display) (`PlayerController.DeprojectScreenPositionToWorld` _returnvalue (/ (`KismetMathLibrary.Conv_IntToDouble` _sizex) 2.0) (/ (`KismetMathLibrary.Conv_IntToDouble` _sizey) 2.0))) false false)
  (if (== (`self.K2_GetActorLocation`) (`self.Damage_Source`) :`ErrorTolerance` 100.0)
    (set `self.Damage_Source` (0.0 0.0 0.0))))

(fn `UserConstructionScript`
  (set `self.Health` (`self.Max_Health`))
  (set `self.Armour` (`self.Max_Armour`)))