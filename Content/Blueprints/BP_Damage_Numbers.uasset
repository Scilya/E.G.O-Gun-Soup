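; BP_Damage_Numbers is a short-lived actor, by its name a floating damage number.
; On BeginPlay its ProjectileMovement launches it upward with a random sideways velocity in local space.
; Each tick it turns to face the deprojected screen-center point of player 0, billboarding toward the view.
; Tick also accumulates LifeSpan and destroys the actor once it reaches one second.
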(event `self.ReceiveBeginPlay`
  (bind _returnvalue (`KismetMathLibrary.RandomFloatInRange` -200.0 200.0))
  (`ProjectileMovementComponent.SetVelocityInLocalSpace` (`self.ProjectileMovement`) (`KismetMathLibrary.MakeVector` _returnvalue _returnvalue 700.0)))

(event `self.ReceiveTick`
  (params (DeltaSeconds :type "Float (single-precision)"))
  (bind _returnvalue (`GameplayStatics.GetPlayerController` 0))
  (bind (_sizex _sizey) (`PlayerController.GetViewportSize` _returnvalue))
  (`self.K2_SetActorRotation` (`KismetMathLibrary.FindLookAtRotation` (`self.K2_GetActorLocation`) (`PlayerController.DeprojectScreenPositionToWorld` _returnvalue (/ (`KismetMathLibrary.Conv_IntToDouble` _sizex) 2.0) (/ (`KismetMathLibrary.Conv_IntToDouble` _sizey) 2.0))))
  (bind _output_get (set `self.Life_Span` (+ (`self.Life_Span`) DeltaSeconds)))
  (if (>= _output_get 1.0)
    (`self.K2_DestroyActor`)))

(fn `UserConstructionScript`)