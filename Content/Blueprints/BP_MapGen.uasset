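; Procedural map generator that, on BeginPlay, builds a tile layout using a weighted random walk north, east or west without direct backtracking.
; Each tile's side-collision overlaps identify its neighbours, and the connection count selects a dead-end, straight, corner, three-way or four-way mesh and rotation.
; One randomly chosen second-half tile becomes the objective and is reported to the HUD, then navigation location and scale are derived before CallTest.
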(event `self.ReceiveBeginPlay`
  (bind _generated_tiles (`self.Generated_Tiles`))
  (bind _returnvalue (`KismetArrayLibrary.Array_Length` _generated_tiles))
  (bind _foundwidgets (`WidgetBlueprintLibrary.GetAllWidgetsOfClass` "/Game/Blueprints/BP_Widget.BP_Widget_C"))
  (for _array_element _foundwidgets
    (set `self.HUD_Ref` _array_element)
    (set `self.Objective_Can_Spawn?` false)
    (for _index (range (+ (`self.Spawn_Tile_Last_Index`) 1))
      (`self.Spawn_Tile` (`|GetArrayItem` (`self.Generated_Tiles`) (- _index 1))))
    (for _index_2 (range (+ _returnvalue 1))
      (bind _output (`|GetArrayItem` _generated_tiles _index_2))
      (`/Engine/EditorBlueprintResources/StandardMacros.IsValid` _output
        (:`Is Valid`
          (`self.Check_Collisions` _output))))
    (for _index_3 (range (+ _returnvalue 1))
      (bind _output_2 (`|GetArrayItem` _generated_tiles _index_3))
      (`/Engine/EditorBlueprintResources/StandardMacros.IsValid` _output_2
        (:`Is Valid`
          (`self.Collisions_Count` _output_2))))
    (for _index_4 (range (+ _returnvalue 1))
      (bind _output_3 (`|GetArrayItem` _generated_tiles _index_4))
      (`/Engine/EditorBlueprintResources/StandardMacros.IsValid` _output_3
        (:`Is Valid`
          (if (and (> _index_4 (/ _returnvalue 2)) (not (`self.Objective_Can_Spawn?`)))
            (set `self.Objective_Can_Spawn?` true))
          (bind _total_collisions (`/Game/Blueprints/BP_Tile.Total_Collisions` _output_3))
          (if (== _total_collisions 1)
            (`self.Spawn_1Way_Tile` _output_3 _index_4)
            (elif (== _total_collisions 2)
              (`self.Spawn_2Way_Tile` _output_3 _index_4)
              (elif (== _total_collisions 3)
                (`self.Spawn_3Way_Tile` _output_3 _index_4)
                (elif (== _total_collisions 4)
                  (`self.Spawn_4Way_Tile` _output_3)
                  (else
                    (`KismetSystemLibrary.PrintString` "ERROR IN MAP GEN")))))))))
    (set `self.Nav_Loc` (/ (+ (`self.K2_GetActorLocation` (`|GetArrayItem` _generated_tiles)) (`self.K2_GetActorLocation` (`|GetArrayItem` _generated_tiles (- _returnvalue 1)))) 2))
    (set `self.Nav_Scale` (`KismetMathLibrary.MakeVector` (`KismetMathLibrary.Conv_IntToDouble` (`self.TEST_INT_2`)) (`KismetMathLibrary.Conv_IntToDouble` (`self.TEST_INT`)) 1.0))
    (`self.Test`)))

(fn `Check_Collisions`
  (params (Tile_Ref :type "/Game/Blueprints/BP_Tile Object Reference"))
  (`self.North_Collisions` Tile_Ref
    (:`false`
      (`self.South_Collisions` Tile_Ref
        (:`false`
          (`self.East_Collisions` Tile_Ref
            (:`false`
              (`self.West_Collisions` Tile_Ref))))))))

(fn `Spawn_Tile`
  (params (Base_Tile :type "/Game/Blueprints/BP_Tile Object Reference"))
  (returns (New_tile :type "/Game/Blueprints/BP_Tile Object Reference"))
  (bind _returnvalue (`self.K2_GetActorLocation` Base_Tile))
  (bind _west_weight (`self.West_Weight`))
  (bind _north_weight (`self.North_Weight`))
  (bind _east_weight (`self.East_Weight`))
  (`/Engine/EditorBlueprintResources/StandardMacros.IsValid` Base_Tile
    (:`Is Valid`
      (bind _output_get (set `self.Rand_Direction` (`KismetMathLibrary.RandomIntegerInRange` (`self.Min_Spawn_Direction`) (`self.Max_Spawn_Direction`))))
      (if (and (== _output_get 0) (< (`self.North_Weight`) 3))
        (set `self.New_Tile_Location` (+ _returnvalue (30000.0 0.0 0.0)) :!label _label)
        (set `self.Prev_East` false)
        (set `self.Prev_West` false)
        (`self.Calc_North_Weight` _north_weight _east_weight _west_weight
          (:`execute`
            (`/Engine/EditorBlueprintResources/StandardMacros.IncrementInt` (`self.TEST_INT_2`)
              (:`  `
                _))))
        (else
          (if (and (== _output_get 1) (not (`self.Prev_West`)) (< (`self.East_Weight`) 3))
            (set `self.New_Tile_Location` (+ _returnvalue (0.0 30000.0 0.0)))
            (set `self.Prev_East` true)
            (set `self.Prev_West` false)
            (`self.Calc_East_Weight` _north_weight _east_weight _west_weight
              (:`execute`
                _))
            (elif (and (not (`self.Prev_East`)) (< (`self.West_Weight`) 3))
              (set `self.New_Tile_Location` (+ _returnvalue (0.0 -30000.0 0.0)))
              (set `self.Prev_East` false)
              (set `self.Prev_West` true)
              (`self.Calc_West_Weight` _north_weight _east_weight _west_weight
                (:`execute`
                  _))
              (else
                (goto _label))))
          (`/Engine/EditorBlueprintResources/StandardMacros.IncrementInt` (`self.TEST_INT`)
            (:`  `
              _)))))
    (:`Is Not Valid`
      (set `self.New_Tile_Location` (0.0 0.0 0.0))))
  (bind _returnvalue_2 (`|SpawnActorFromClass` "/Game/Blueprints/BP_Tile.BP_Tile_C" (`KismetMathLibrary.MakeTransform` (`self.New_Tile_Location`)) "Undefined" "OverrideRootScale" null null))
  (`KismetArrayLibrary.Array_Add` (`self.Generated_Tiles`) _returnvalue_2)
  (return null))

(fn `UserConstructionScript`)