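; BP_Interactable_MissionStart is an interactable that starts the selected mission, or prints a warning when none is selected.
; On interact it loads or creates the BP_GameStats save in the GameStats slot, writes SelectedMission into CurrentMission and saves it.
; It then clears all widgets, shows the BP_Loading screen and opens the hardcoded Test_Map level, so the save object carries the mission choice across the level change.
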(event `self.OnInteract`
  (params (`Interacting Actor` :type "Actor Object Reference"))
  (bind _gamestats_ref (`self.GameStats_Ref`))
  (if (`KismetStringLibrary.EqualEqual_StrStr` (`self.Selected_Mission`) "NoMission")
    (`KismetSystemLibrary.PrintString` "You have not selected a Mission")
    (else
      (bind _returnvalue (`GameplayStatics.DoesSaveGameExist` "GameStats"))
      (if _returnvalue
        (bind _returnvalue_2 (`GameplayStatics.LoadGameFromSlot` "GameStats"))
        (bind _asbp_game_stats (cast `/Game/Blueprints/BP_GameStats` _returnvalue_2))
        (set `self.GameStats_Ref` _asbp_game_stats)
        (else
          (bind _returnvalue_3 (`GameplayStatics.CreateSaveGameObject` "/Game/Blueprints/BP_GameStats.BP_GameStats_C"))
          (set `self.GameStats_Ref` _returnvalue_3)))
      (set `/Game/Blueprints/BP_GameStats.Current_Mission` (`self.Selected_Mission`) _gamestats_ref)
      (`GameplayStatics.SaveGameToSlot` _gamestats_ref "GameStats")
      (`WidgetLayoutLibrary.RemoveAllWidgets`)
      (bind _returnvalue_4 (`|CreateWidget` "/Game/Blueprints/BP_Loading.BP_Loading_C" (`GameplayStatics.GetPlayerController` 0)))
      (`UserWidget.AddToViewport` _returnvalue_4 0)
      (`GameplayStatics.OpenLevel` "Test_Map"))))

(fn `UserConstructionScript`
  (`parent.UserConstructionScript`))