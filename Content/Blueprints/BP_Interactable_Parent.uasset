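; BP_Interactable_Parent is a base Blueprint for interactable objects, with an empty OnInteract event that receives the interacting actor.
; Each tick, it turns its Widget component toward the world location deprojected from the center of the first player's viewport, so it faces the view.
; It then hides the widget every frame without propagating to children, so nothing in this graph makes it visible.
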(event `OnInteract`
  (params (`Interacting Actor` :type "Actor Object Reference")))

(event `self.ReceiveTick`
  (params (DeltaSeconds :type "Float (single-precision)"))
  (bind _returnvalue (`GameplayStatics.GetPlayerController` 0))
  (bind _widget (`self.Widget`))
  (bind (_sizex _sizey) (`PlayerController.GetViewportSize` _returnvalue))
  (`SceneComponent.K2_SetWorldRotation` _widget (`KismetMathLibrary.FindLookAtRotation` (`SceneComponent.K2_GetComponentLocation` _widget) (`PlayerController.DeprojectScreenPositionToWorld` _returnvalue (/ (`KismetMathLibrary.Conv_IntToDouble` _sizex) 2.0) (/ (`KismetMathLibrary.Conv_IntToDouble` _sizey) 2.0))) false false)
  (`SceneComponent.SetVisibility` _widget false false))

(fn `UserConstructionScript`)