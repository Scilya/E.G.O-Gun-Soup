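; BP_DropPod is an enemy delivery actor that spawns one AI enemy on contact with the map, then destroys itself.
; BeginPlay randomly picks the small, medium or large enemy class; the boss entry in the class list is outside that range.
; When its Box overlaps a component whose display name contains "Map", it spawns the pawn with BT_Enemy slightly above the Cube's location.
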(event `self.ReceiveBeginPlay`
  (set `self.EnemySpawnType` (`KismetMathLibrary.RandomIntegerInRange` 0 2)))

(event `self.Box.OnComponentBeginOverlap`
  (params (OverlappedComponent :type "PrimitiveComponent Object Reference") (OtherActor :type "Actor Object Reference") (OtherComp :type "PrimitiveComponent Object Reference") (OtherBodyIndex :type Integer) (bFromSweep :type Boolean) (SweepResult :type "HitResult Structure (by ref)"))
  (bind (_returnvalue_x _returnvalue_y _returnvalue_z) (`KismetMathLibrary.BreakVector` (`SceneComponent.K2_GetComponentLocation` (`self.Cube`))))
  (if (`KismetStringLibrary.Contains` (`KismetSystemLibrary.GetDisplayName` OtherComp) "Map")
    (`AIBlueprintHelperLibrary.SpawnAIFromClass` (`|GetArrayItem` (`|MakeArray` "/Game/AI/BP_Enemy_S.BP_Enemy_S_C" "/Game/AI/BP_Enemy_M.BP_Enemy_M_C" "/Game/AI/BP_Enemy_L.BP_Enemy_L_C" "/Game/AI/BP_Enemy_Boss.BP_Enemy_Boss_C" :!type "Pawn Class Reference") (`self.EnemySpawnType`)) "/Game/AI/BT_Enemy.BT_Enemy" (`KismetMathLibrary.MakeVector` _returnvalue_x _returnvalue_y (+ _returnvalue_z 50.0)))
    (`self.K2_DestroyActor`)))

(fn `UserConstructionScript`)