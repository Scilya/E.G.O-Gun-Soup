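; Player character with mouse-look movement and hitscan rifle, shotgun and sniper weapons, including sniper scope zoom.
; Weapon-mode macros deproject screen centre for automatic, multi-pellet or single shots and roll tiered crits above 100% chance.
; A shared trace applies impulses, destructible damage, decals, or armour-scaled enemy damage with neck-bone headshots and coloured damage numbers.
; Reloads start through BP_Widget and refill ammo when Reload_Complete fires.
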(event `self.ReceiveBeginPlay`
  (set `CharacterMovementComponent.MaxWalkSpeed` 4000.0 (`self.CharacterMovement`))
  (if (`self.Sniper?`)
    (set `self.Curr_Weapon_Ammo` (`self.Curr_Ammo_Sniper`))
    (set `self.Max_Weapon_Ammo` (`self.Max_Ammo_Sniper`))
    (elif (`self.Shotgun?`)
      (set `self.Curr_Weapon_Ammo` (`self.Curr_Ammo_Shotgun`))
      (set `self.Max_Weapon_Ammo` (`self.Max_Ammo_Shotgun`))
      (else
        (set `self.Curr_Weapon_Ammo` (`self.Curr_Ammo_Rifle`))
        (set `self.Max_Weapon_Ammo` (`self.Max_Ammo_Rifle`))))))

(event `InputAxisKey|MouseX`
  (params (AxisValue :type "Float (single-precision)"))
  (bind _cube1 (`self.Cube1`))
  (`SceneComponent.K2_SetRelativeRotation` _cube1 (`KismetMathLibrary.MakeRotator` (.roll (`SceneComponent.RelativeRotation` _cube1)) (.pitch (`SceneComponent.RelativeRotation` _cube1)) (+ AxisValue (.yaw (`SceneComponent.RelativeRotation` _cube1)))) false false))

(event `InputAxisKey|MouseY`
  (params (AxisValue :type "Float (single-precision)"))
  (bind _cube1 (`self.Cube1`))
  (`SceneComponent.K2_SetRelativeRotation` _cube1 (`KismetMathLibrary.MakeRotator` (.roll (`SceneComponent.RelativeRotation` _cube1)) (`KismetMathLibrary.ClampAngle` (+ AxisValue (.pitch (`SceneComponent.RelativeRotation` _cube1))) -85.0 85.0) (.yaw (`SceneComponent.RelativeRotation` _cube1))) false false))

(event `self.ReceiveTick`
  (params (DeltaSeconds :type "Float (single-precision)"))
  (bind _fire_timer (`self.Fire_Timer`))
  (if (> _fire_timer 0.0)
    (set `self.Fire_Timer` (- _fire_timer 0.1))))

(event `InputAxis|Move_X`
  (params (AxisValue :type "Float (single-precision)"))
  (bind _mesh (`self.Mesh`))
  (bind (_relativerotation_roll _relativerotation_pitch) (`KismetMathLibrary.BreakRotator` (`SceneComponent.RelativeRotation` _mesh)))
  (bind (_relativerotation_roll_2 _relativerotation_pitch_2 _relativerotation_yaw) (`KismetMathLibrary.BreakRotator` (`SceneComponent.RelativeRotation` (`self.Cube1`))))
  (`self.AddMovementInput` (`KismetMathLibrary.GetForwardVector` (`KismetMathLibrary.MakeRotator` 0.0 0.0 (.yaw (`SceneComponent.RelativeRotation` (`self.Cube1`))))) AxisValue)
  (`SceneComponent.K2_SetRelativeRotation` _mesh (`KismetMathLibrary.MakeRotator` _relativerotation_roll _relativerotation_pitch (- _relativerotation_yaw 90.0)) false false))

(event `InputAxis|Move_Y`
  (params (AxisValue :type "Float (single-precision)"))
  (`self.AddMovementInput` (`KismetMathLibrary.GetRightVector` (`KismetMathLibrary.MakeRotator` 0.0 0.0 (.yaw (`SceneComponent.RelativeRotation` (`self.Cube1`))))) AxisValue))

(event `InputAction|Shoot`
  (params (Key :type "Key Structure"))
  (bind _hitscan_end (`self.Hitscan_End`))
  (bind _curr_weapon_ammo (`self.Curr_Weapon_Ammo`))
  (bind _returnvalue (`SceneComponent.K2_GetComponentLocation` (`self.Cube1`)))
  (bind _returnvalue_2 (not (`self.Reloading?`)))
  (bind _returnvalue_3 (and (`KismetMathLibrary.InRange_IntInt` _curr_weapon_ammo 0 (`self.Max_Weapon_Ammo`) false) _returnvalue_2))
  (:`Pressed`
    (if _returnvalue_3
      (if (<= (`self.Fire_Timer`) 0.0)
        (if (`self.Sniper?`)
          (`self.Sniper_Mode`)
          (`/Engine/EditorBlueprintResources/StandardMacros.DecrementInt` _curr_weapon_ammo :!label _label
            (:`  `
              (bind (_outhit _returnvalue_4) (`KismetSystemLibrary.LineTraceSingle` (`self.Hitscan_Start`) _hitscan_end "TraceTypeQuery1" true :!label _label_2))
              (if _returnvalue_4
                (bind (_bblockinghit _binitialoverlap _time _distance _location _impactpoint _normal _impactnormal _physmat _hitactor _hitcomponent _hitbonename) (`GameplayStatics.BreakHitResult` _outhit))
                (bind _output_get (set `self.Reticle_Target` _location))
                (else
                  (set `self.Reticle_Target` _hitscan_end)))
              (`KismetSystemLibrary.DrawDebugLine` _returnvalue _output_get (struct :`R` 0.57 :`G` 0.008849 :`A` 1.0) 0.1 8.0)
              (set `self.Distance_M` (`KismetMathLibrary.FTrunc` (/ (`KismetMathLibrary.VSize` (- _returnvalue _output_get)) 1000.0)))
              (`/Engine/EditorBlueprintResources/StandardMacros.IsValid` _hitcomponent
                (:`Is Valid`
                  (if (`SceneComponent.IsSimulatingPhysics` _hitcomponent "None")
                    (bind _returnvalue_5 (`KismetMathLibrary.Normal` (`KismetMathLibrary.GetDirectionUnitVector` _returnvalue _output_get)))
                    (`PrimitiveComponent.AddImpulse` _hitcomponent (* _returnvalue_5 500000) _hitbonename false))
                  (bind _returnvalue_6 (`KismetSystemLibrary.GetDisplayName` _hitcomponent))
                  (if (`KismetStringLibrary.Contains` _returnvalue_6 "Destructible")
                    (bind _asdestructible_component (cast `DestructibleComponent` _hitcomponent))
                    (`DestructibleComponent.ApplyDamage` _asdestructible_component 1.0 (`self.Reticle_Target`) _returnvalue_5 1.0)
                    (elif (`KismetStringLibrary.Contains` _returnvalue_6 "Enemy")
                      (bind _asbp_enemy_parent (cast `/Game/AI/BP_Enemy_Parent` _hitactor)
                        (:`then`
                          (bind _returnvalue_7 (`self.Enemy_Damage_Calc` _asbp_enemy_parent (`KismetStringLibrary.Contains` (`KismetStringLibrary.Conv_NameToString` _hitbonename) "Neck"))
                            (:`  `
                              (bind _output_get_2 (set `/Game/AI/BP_Enemy_Parent.Health` _returnvalue_7 _asbp_enemy_parent))
                              (bind _asbp_enemy_widget (cast `/Game/Blueprints/BP_Enemy_Widget` (`WidgetComponent.GetUserWidgetObject` (`/Game/AI/BP_Enemy_Parent.Health_Display` _asbp_enemy_parent))))
                              (`/Game/Blueprints/BP_Enemy_Widget.Enemy_Health` _asbp_enemy_widget _output_get_2 (`/Game/AI/BP_Enemy_Parent.Max_Health` _asbp_enemy_parent))
                              (bind _returnvalue_8 (`|SpawnActorFromClass` "/Game/Blueprints/BP_Damage_Numbers.BP_Damage_Numbers_C" (`KismetMathLibrary.MakeTransform` (`self.Reticle_Target`)) "Undefined" "OverrideRootScale" null null))
                              (bind _textrender (`/Game/Blueprints/BP_Damage_Numbers.TextRender` _returnvalue_8))
                              (`TextRenderComponent.K2_SetText` _textrender (`KismetTextLibrary.Conv_IntToText` (`self.Damage_Done`)))
                              (if (`self.Crit?`)
                                (if (`self.Orange_Crit?`)
                                  (if (`self.Red_Crit?`)
                                    (set `self.Damage_Colour` (make `Color` 0 0 255))
                                    (set `self.Damage_Size` 80.0)
                                    (else
                                      (set `self.Damage_Colour` (make `Color` 0 100 255))
                                      (set `self.Damage_Size` 70.0)))
                                  (else
                                    (set `self.Damage_Colour` (make `Color` 0 255 255))
                                    (set `self.Damage_Size` 60.0)))
                                (else
                                  (set `self.Damage_Colour` (make `Color` 255 255 255))
                                  (set `self.Damage_Size` 50.0)))
                              (`TextRenderComponent.SetTextRenderColor` _textrender (`self.Damage_Colour`))
                              (`TextRenderComponent.SetWorldSize` _textrender (`self.Damage_Size`)))))
                        (:`CastFailed`
                          (`KismetSystemLibrary.PrintString` "Enemy Cast Failed")))
                      (else
                        (bind _returnvalue_9 (`GameplayStatics.SpawnDecalAtLocation` "/Game/Materials/M_Bullet_Decal.M_Bullet_Decal" (25.0 25.0 25.0) (`self.Reticle_Target`) (`KismetMathLibrary.Conv_VectorToRotator` _impactnormal) 20.0))
                        (`DecalComponent.SetFadeScreenSize` _returnvalue_9 0.002))))))))
          (elif (`self.Shotgun?`)
            (`self.Shotgun_Mode`
              (:`then`
                (goto _label_2))
              (:`Loop Complete`
                (goto _label)))
            (else
              (`self.Rifle_Mode` _returnvalue_3 :!label _label_3
                (:`then`
                  (goto _label))
                (:`No Ammo`
                  (if (and (== _curr_weapon_ammo 0) _returnvalue_2) :!label _label_4
                    (if (not (or (`self.Reloading?`) (== (`self.Curr_Weapon_Ammo`) (`self.Max_Weapon_Ammo`)))) :!label _label_5
                      (bind _foundwidgets (`WidgetBlueprintLibrary.GetAllWidgetsOfClass` "/Game/Blueprints/BP_Widget.BP_Widget_C"))
                      (for _array_element _foundwidgets
                        (`/Game/Blueprints/BP_Widget.Reload` _array_element (`self.Reload_Speed`))
                        (set `self.Reloading?` true)
                        (goto _label_6 :!via `Reset`))))))))))
      (else
        (goto _label_4))))
  (:`Released`
    (goto _label_3 :!via `Released`)))

(event `InputAction|TEST_SHOTGUN`
  (params (Key :type "Key Structure"))
  (:`Pressed`
    (`self.Shotgun_Mode`
      (:`then`
        (goto _label_2)))))

(event `InputAction|Reload`
  (params (Key :type "Key Structure"))
  (:`Pressed`
    (goto _label_5)))

(event `Reload_Complete`
  (`/Engine/EditorBlueprintResources/StandardMacros.DoOnce` false :!label _label_6
    (:`Completed`
      (set `self.Curr_Weapon_Ammo` (`self.Max_Weapon_Ammo`))
      (if (`self.Sniper?`)
        (set `self.Curr_Ammo_Sniper` (`self.Max_Ammo_Sniper`))
        (elif (`self.Shotgun?`)
          (set `self.Curr_Ammo_Shotgun` (`self.Max_Ammo_Shotgun`))
          (else
            (set `self.Curr_Ammo_Rifle` (`self.Max_Ammo_Rifle`)))))
      (set `self.Reloading?` false))))

(event `InputAction|ADS`
  (params (Key :type "Key Structure"))
  (bind _camera (`self.Camera`))
  (:`Pressed`
    (if (`self.Sniper?`)
      (set `self.Scope_Alpha` 1.0)
      (`CameraComponent.SetFieldOfView` _camera 10.0)
      (bind _foundwidgets (`WidgetBlueprintLibrary.GetAllWidgetsOfClass` "/Game/Blueprints/BP_Widget.BP_Widget_C" :!label _label_7))
      (for _array_element _foundwidgets
        (`/Game/Blueprints/BP_Widget.ADS` _array_element (`self.Scope_Alpha`)))))
  (:`Released`
    (set `self.Scope_Alpha` 0.0)
    (`CameraComponent.SetFieldOfView` _camera 90.0)
    (goto _label_7)))

(fn `UserConstructionScript`)