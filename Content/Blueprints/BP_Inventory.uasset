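; BP_Inventory stores the data for one modular gun, apparently as an inventory record of a weapon.
; It holds a mesh and material for barrel, receiver and magazine, plus combat stats, rarity, and automatic and scoped properties.
; A setter writes all these variables at once and a getter returns them together, with no other logic.
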(fn `Get_Inv_Variables`
  (returns (BarrelMesh :type "SkeletalMesh Object Reference") (ReceiverMesh :type "SkeletalMesh Object Reference") (MagazineMesh :type "SkeletalMesh Object Reference") (BarrelMat :type "MaterialInstance Object Reference") (ReceiverMat :type "MaterialInstance Object Reference") (MagazineMat :type "MaterialInstance Object Reference") (Damage :type "Float (double-precision)") (CritChance :type "Float (double-precision)") (CritDamage :type "Float (double-precision)") (FireRate :type "Float (double-precision)") (Spread :type "Float (double-precision)") (Multishot :type Integer) (Rarity :type Integer) (`Auto?` :type Boolean) (Scoped :type Boolean))
  (return (`self.BarrelMesh`) (`self.ReceiverMesh`) (`self.MagazineMesh`) (`self.BarrelMat`) (`self.ReceiverMat`) (`self.MagazineMat`) (`self.Damage`) (`self.CritChance`) (`self.CritDamage`) (`self.FireRate`) (`self.Spread`) (`self.Multishot`) (`self.Rarity`) (`self.Auto?`) (`self.Scoped`)))

(fn `Set_Inv_Variables`
  (params (BarrelMesh :type "SkeletalMesh Object Reference") (ReceiverMesh :type "SkeletalMesh Object Reference") (MagazineMesh :type "SkeletalMesh Object Reference") (BarrelMat :type "MaterialInstance Object Reference") (ReceiverMat :type "MaterialInstance Object Reference") (MagazineMat :type "MaterialInstance Object Reference") (Damage :type "Float (double-precision)") (CritChance :type "Float (double-precision)") (CritDamage :type "Float (double-precision)") (FireRate :type "Float (double-precision)") (Spread :type "Float (double-precision)") (Multishot :type Integer) (Rarity :type Integer) (`Auto?` :type Boolean) (Scoped :type Boolean))
  (set `self.BarrelMesh` BarrelMesh)
  (set `self.ReceiverMesh` ReceiverMesh)
  (set `self.MagazineMesh` MagazineMesh)
  (set `self.BarrelMat` BarrelMat)
  (set `self.ReceiverMat` ReceiverMat)
  (set `self.MagazineMat` MagazineMat)
  (set `self.Damage` Damage)
  (set `self.CritChance` CritChance)
  (set `self.CritDamage` CritDamage)
  (set `self.FireRate` FireRate)
  (set `self.Spread` Spread)
  (set `self.Multishot` Multishot)
  (set `self.Rarity` Rarity)
  (set `self.Auto?` `Auto?`)
  (set `self.Scoped` Scoped))