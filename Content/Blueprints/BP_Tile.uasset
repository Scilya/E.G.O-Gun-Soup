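; BP_Tile is a map tile that spawns drop pods when the player first enters it.
; Overlapping its Box with an actor whose display name contains "Player" fires a DoOnce, spawning three BP_DropPod actors at random points inside SpawnVolume.
; An unconnected graph section would place random small or large destructible buildings on shuffled corner nodes, but never runs.
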(event `self.Box.OnComponentBeginOverlap`
  (params (OverlappedComponent :type "PrimitiveComponent Object Reference") (OtherActor :type "Actor Object Reference") (OtherComp :type "PrimitiveComponent Object Reference") (OtherBodyIndex :type Integer) (bFromSweep :type Boolean) (SweepResult :type "HitResult Structure (by ref)"))
  (bind _spawn_volume (`self.Spawn_Volume`))
  (bind _x (.x (`BoxComponent.GetScaledBoxExtent` _spawn_volume)))
  (bind _y (.y (`BoxComponent.GetScaledBoxExtent` _spawn_volume)))
  (bind _z (.z (`BoxComponent.GetScaledBoxExtent` _spawn_volume)))
  (if (`KismetStringLibrary.Contains` (`KismetSystemLibrary.GetDisplayName` OtherActor) "Player")
    (`/Engine/EditorBlueprintResources/StandardMacros.DoOnce` false
      (:`Completed`
        (for _ (range 3)
          (`|SpawnActorFromClass` "/Game/Blueprints/BP_DropPod.BP_DropPod_C" (`KismetMathLibrary.MakeTransform` (+ (`KismetMathLibrary.MakeVector` (`KismetMathLibrary.RandomFloatInRange` (* _x -1.0) _x) (`KismetMathLibrary.RandomFloatInRange` (* _y -1.0) _y) (`KismetMathLibrary.RandomFloatInRange` (* _z -1.0) _z)) (`SceneComponent.K2_GetComponentLocation` _spawn_volume))) "Undefined" "OverrideRootScale" null null))))))

(event `self.Map_Tile.OnComponentActivated`
  (params (Component :type "ActorComponent Object Reference") (bReset :type Boolean)))

(fn `UserConstructionScript`)