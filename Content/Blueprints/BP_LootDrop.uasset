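; BP_LootDrop is a loot pickup that launches with a random impulse and takes on a random rarity look when it spawns.
; On BeginPlay, successive random rolls against thresholds scaled by LootMultiplier pick Exotic, Rare, Uncommon or Common.
; That tier sets the mesh material, billboard glow, particle template and point light colour.
; The LootChance text shows a separate random number, unrelated to the rarity rolls.
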(event `self.ReceiveBeginPlay`
  (bind _returnvalue (`KismetMathLibrary.RandomFloatInRange` 0.0 100.0))
  (bind _returnvalue_2 (`KismetMathLibrary.RandomFloatInRange` -100000.0 100000.0))
  (bind _loot_multiplier (`self.Loot_Multiplier`))
  (`PrimitiveComponent.AddImpulse` (`self.Loot`) (`KismetMathLibrary.MakeVector` _returnvalue_2 _returnvalue_2 (`KismetMathLibrary.RandomFloatInRange` 100000.0 150000.0)) "None" false)
  (if (< _returnvalue (* _loot_multiplier 0.1))
    (set `self.Loot_Material` "/Game/Materials/M_Exotic.M_Exotic")
    (set `self.Glow_Material` "/Game/Materials/M_Glow_Exotic.M_Glow_Exotic")
    (set `self.Glow_Particle` "/Game/Assets/P_LootGlow_Exotic.P_LootGlow_Exotic")
    (set `self.Light_Colour` (struct :`R` 1.0 :`G` 0.216 :`A` 1.0))
    (elif (< _returnvalue (* _loot_multiplier 0.9))
      (set `self.Loot_Material` "/Game/Materials/M_Rare.M_Rare")
      (set `self.Glow_Material` "/Game/Materials/M_Glow_Rare.M_Glow_Rare")
      (set `self.Glow_Particle` "/Game/Assets/P_LootGlow_Rare.P_LootGlow_Rare")
      (set `self.Light_Colour` (struct :`R` 0.473958 :`B` 0.415199 :`A` 1.0))
      (elif (< _returnvalue (* _loot_multiplier 9.0))
        (set `self.Loot_Material` "/Game/Materials/M_Uncommon.M_Uncommon")
        (set `self.Glow_Material` "/Game/Materials/M_Glow_Uncommon.M_Glow_Uncommon")
        (set `self.Glow_Particle` "/Game/Assets/P_LootGlow_Uncommon.P_LootGlow_Uncommon")
        (set `self.Light_Colour` (struct :`G` 0.53125 :`B` 0.53125 :`A` 1.0))
        (else
          (set `self.Loot_Material` "/Game/Materials/M_Common.M_Common")
          (set `self.Glow_Material` "/Game/Materials/M_Glow_Common.M_Glow_Common")
          (set `self.Glow_Particle` "/Game/Assets/P_LootGlow_Common.P_LootGlow_Common")
          (set `self.Light_Colour` (struct :`R` 1.0 :`G` 1.0 :`B` 1.0 :`A` 1.0))))))
  (`PrimitiveComponent.SetMaterial` (`self.Loot`) 0 (`self.Loot_Material`))
  (`PrimitiveComponent.SetMaterial` (`self.MaterialBillboard`) 0 (`self.Glow_Material`))
  (`ParticleSystemComponent.SetTemplate` (`self.P_LootGlow`) (`self.Glow_Particle`))
  (`LightComponent.SetLightColor` (`self.PointLight`) (`self.Light_Colour`) true)
  (`TextRenderComponent.K2_SetText` (`self.Loot_Chance`) (`KismetTextLibrary.Conv_DoubleToText` _returnvalue "HalfToEven")))

(fn `UserConstructionScript`)