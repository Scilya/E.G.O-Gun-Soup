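; BP_Projectile is a projectile that damages destructibles and light enemies when its Sphere begins overlapping them.
; It tells targets apart by substrings in the overlapped component's display name, ignoring "Player" and any unmatched names.
; Destructible components receive damage with a directional impulse, while BP_Enemy_Light loses Health scaled down by its Armour.
; The projectile destroys itself after applying either kind of hit.
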(event `self.Sphere.OnComponentBeginOverlap`
  (params (OverlappedComponent :type "PrimitiveComponent Object Reference") (OtherActor :type "Actor Object Reference") (OtherComp :type "PrimitiveComponent Object Reference") (OtherBodyIndex :type Integer) (bFromSweep :type Boolean) (SweepResult :type "HitResult Structure (by ref)"))
  (bind _returnvalue (`KismetSystemLibrary.GetDisplayName` OtherComp))
  (bind (_bblockinghit _binitialoverlap _time _distance _location _impactpoint _normal _impactnormal _physmat _hitactor) (`GameplayStatics.BreakHitResult` SweepResult))
  (if (`KismetStringLibrary.Contains` (`KismetSystemLibrary.GetDisplayName` OtherComp) "Player")
    _
    (elif (`KismetStringLibrary.Contains` _returnvalue "Destructible")
      (bind _asdestructible_component (cast `DestructibleComponent` OtherComp))
      (`DestructibleComponent.ApplyDamage` _asdestructible_component 10.0 _impactpoint (* (`KismetMathLibrary.Normal` (`KismetMathLibrary.GetDirectionUnitVector` _impactpoint _location)) 5000000) 10.0)
      (`self.K2_DestroyActor`)
      (elif (`KismetStringLibrary.Contains` _returnvalue "Enemy")
        (bind _asbp_enemy_light (cast `/Game/AI/BP_Enemy_Light` _hitactor))
        (set `/Game/AI/BP_Enemy_Light.Health` (- (`/Game/AI/BP_Enemy_Light.Health` _asbp_enemy_light) (* 100.0 (/ 300.0 (`KismetMathLibrary.Conv_IntToDouble` (+ (`/Game/AI/BP_Enemy_Light.Armour` _asbp_enemy_light) 300))))) _asbp_enemy_light)
        (`self.K2_DestroyActor`)))))

(fn `UserConstructionScript`)