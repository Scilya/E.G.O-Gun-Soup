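; Interactable weapon loot drop that launches with a random upward impulse on spawn and shows the rarity of the weapon it carries.
; On BeginPlay it reads Rarity from the GeneratedWeapon child actor to set the loot material, glow billboard, particle and light colour.
; When a Player-tagged actor interacts, it passes the weapon and itself to BP_Player's WeaponAdd.
; Its Weapon_PickedUp event destroys the drop.
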(event `self.ReceiveBeginPlay`
  (bind _returnvalue (`KismetMathLibrary.RandomFloatInRange` -100000.0 100000.0))
  (`PrimitiveComponent.AddImpulse` (`self.Loot`) (`KismetMathLibrary.MakeVector` _returnvalue _returnvalue (`KismetMathLibrary.RandomFloatInRange` 200000.0 250000.0)) "None" false)
  (bind _asweapon_generation_test (cast `/Game/Actors/WeaponGenerationTest` (`ChildActorComponent.ChildActor` (`self.Generated_Weapon`))))
  (bind _rarity (`/Game/Actors/WeaponGenerationTest.Rarity` _asweapon_generation_test))
  (if (== _rarity 3)
    (set `self.Loot_Material` "/Game/Materials/M_Exotic.M_Exotic")
    (set `self.Glow_Material` "/Game/Materials/M_Glow_Exotic.M_Glow_Exotic")
    (set `self.Glow_Particle` "/Game/Assets/P_LootGlow_Exotic.P_LootGlow_Exotic")
    (set `self.Light_Colour` (struct :`R` 1.0 :`G` 0.216 :`A` 1.0))
    (elif (== _rarity 2)
      (set `self.Loot_Material` "/Game/Materials/M_Rare.M_Rare")
      (set `self.Glow_Material` "/Game/Materials/M_Glow_Rare.M_Glow_Rare")
      (set `self.Glow_Particle` "/Game/Assets/P_LootGlow_Rare.P_LootGlow_Rare")
      (set `self.Light_Colour` (struct :`R` 0.473958 :`B` 0.415199 :`A` 1.0))
      (elif (== _rarity 1)
        (set `self.Loot_Material` "/Game/Materials/M_Uncommon.M_Uncommon")
        (set `self.Glow_Material` "/Game/Materials/M_Glow_Uncommon.M_Glow_Uncommon")
        (set `self.Glow_Particle` "/Game/Assets/P_LootGlow_Uncommon.P_LootGlow_Uncommon")
        (set `self.Light_Colour` (struct :`G` 0.53125 :`B` 0.53125 :`A` 1.0))
        (else
          (set `self.Loot_Material` "/Game/Materials/M_Common.M_Common")
          (set `self.Glow_Material` "/Game/Materials/M_Glow_Common.M_Glow_Common")
          (set `self.Glow_Particle` "/Game/Assets/P_LootGlow_Common.P_LootGlow_Common")
          (set `self.Light_Colour` (struct :`R` 1.0 :`G` 1.0 :`B` 1.0 :`A` 1.0))))))
  (`PrimitiveComponent.SetMaterial` (`self.Loot`) 0 (`self.Loot_Material`))
  (`PrimitiveComponent.SetMaterial` (`self.MaterialBillboard`) 0 (`self.Glow_Material`))
  (`ParticleSystemComponent.SetTemplate` (`self.P_LootGlow`) (`self.Glow_Particle`))
  (`LightComponent.SetLightColor` (`self.PointLight`) (`self.Light_Colour`) true))

(event `self.OnInteract`
  (params (`Interacting Actor` :type "Actor Object Reference"))
  (if (`self.ActorHasTag` `Interacting Actor` "Player")
    (bind _asbp_player (cast `/Game/Blueprints/BP_Player` `Interacting Actor`))
    (`/Game/Blueprints/BP_Player.Weapon_Add` _asbp_player (`ChildActorComponent.ChildActor` (`self.Generated_Weapon`)) self)))

(event `Weapon_PickedUp`
  (`self.K2_DestroyActor`))

(fn `UserConstructionScript`
  (`parent.UserConstructionScript`))